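; Missile projectile actor that flies forward and damages actors tagged "Target" on contact.
; Tick moves it along local X at FMissileSpeed, scaled by delta time and without sweeping.
; Overlapping a Target applies fixed damage, spawns BP_Explosion at the 폭발효과위치 (explosion effect position) component, and destroys the missile.
; The "Cube" tag branch is empty, and a direct particle emitter spawn is left unconnected.
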(event EventBeginPlay)

(event Collision|EventActorBeginOverlap
  (params (OtherActor :type Actor%20Object%20Reference))
  (Variables|Default|SetOther%20Actor OtherActor)
  (if (Actor|ActorHasTag (Variables|Default|GetOther%20Actor) "Target")
    (Game|Damage|ApplyDamage (Variables|Default|GetOther%20Actor) 1e+01 (Game|GetInstigatorController) self "/Game/Blueprints/BP_DamageType.BP_DamageType_C")
    (Game|SpawnActorfromClass "/Game/Blueprints/BP_Explosion.BP_Explosion_C" (Transformation|GetWorldTransform (Variables|Default|Get폭발효과위치)) "Undefined" 0 0)
    (Actor|DestroyActor)
    (elif (Actor|ActorHasTag (Variables|Default|GetOther%20Actor) "Cube")
      _)))

(event EventTick
  (params (DeltaSeconds :type Float%20%28single-precision%29))
  (Transformation|AddActorLocalOffset (Math|Vector|MakeVector (* DeltaSeconds (Variables|Default|GetfMissile_Speed)) 0.0 0.0) false false))

(event Collision|EventActorEndOverlap
  (params (OtherActor :type Actor%20Object%20Reference)))

(fn ConstructionScript)