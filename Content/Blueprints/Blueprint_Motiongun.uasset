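; Motion gun Blueprint that spins continuously while firing missiles from four fire points.
; Each Tick, MotionGunRotation yaws the Base component by FGunsSpeed scaled by delta time.
; SpawnMissile then spawns a BP_Missile at the world transform of each FirePosition component.
; Firing has no timer or cooldown, so four missiles spawn every frame and the fire rate follows frame rate.
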(event EventBeginPlay)

(event EventTick
  (params (DeltaSeconds :type Float%20%28single-precision%29))
  (CallFunction|MotionGunRotation DeltaSeconds) ; 모션건 회전 함수
  (CallFunction|SpawnMissile (Variables|Default|GetFirePosition1)) ; 미사일 스폰 함수
  (CallFunction|SpawnMissile (Variables|Default|GetFirePosition2))
  (CallFunction|SpawnMissile (Variables|Default|GetFirePosition3))
  (CallFunction|SpawnMissile (Variables|Default|GetFirePosition4)))

(fn ConstructionScript)

(fn MotionGunRotation
  (params (Delta%20Seconds :type Float%20%28single-precision%29))
  (Transformation|AddLocalRotation (Variables|Default|GetBase) (Math|Rotator|MakeRotator 0.0 0.0 (* Delta%20Seconds (Variables|Default|GetfGuns_Speed))) false false))

(fn SpawnMissile
  (params (FirePosition :type Child%20Actor%20Component%20Object%20Reference))
  (Game|SpawnActorfromClass "/Game/Blueprints/BP_Missile.BP_Missile_C" (Transformation|GetWorldTransform FirePosition) "Undefined" 0 0))