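; BGM1 is a background music Blueprint that drives an AudioComponent according to the game's state.
; BeginPlay assigns the MainMenu sound.
; Every Tick casts the game state to MyGameStateBase1 and switches on 현재게임상태, checking the current sound against BGM1 for 탐험 (exploration) and BGM2 for 전투 (battle).
; On a mismatch it calls SetSound, though neither of those calls specifies a sound.
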(event EventBeginPlay
  (Audio|Components|Audio|SetSound (Variables|Components|GetAudioComponent) "/Game/BGM/Main-Menu.Main-Menu"))

(event EventTick
  (params (DeltaSeconds :type Float%20%28single-precision%29))
  (bind _asmy_game_state_base_1 (Utilities|Casting|CastToMyGameStateBase1 (Game|GetGameState)))
  (switch Utilities|FlowControl|Switch|Switchonenum_GameState (Variables|/Game/Blueprints/WorldSettings/MyGameStateBase1.MyGameStateBase1_C|Get현재게임상태 _asmy_game_state_base_1)
    (:NewEnumerator0
      (if (!= (Variables|/Script/Engine.AudioComponent|GetSound (Variables|Components|GetAudioComponent)) "BGM1")
        (Audio|Components|Audio|SetSound (Variables|Components|GetAudioComponent) 0)))
    (:NewEnumerator1
      (if (!= (Variables|/Script/Engine.AudioComponent|GetSound (Variables|Components|GetAudioComponent)) "/Game/Blueprints/Sound/BGM2.BGM2")
        (Audio|Components|Audio|SetSound (Variables|Components|GetAudioComponent) 0)))))

(fn ConstructionScript)