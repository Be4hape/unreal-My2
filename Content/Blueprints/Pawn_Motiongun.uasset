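; Player-controlled gun pawn that swivels on its base and fires a volley of BP_Missile actors.
; Tick yaws the base from the Pawn_Rotation axis and PlayerSpeed, then sets world rotation through a clamp macro meant to limit it to ±30°.
; Pawn_Fire plays audio, spawns a missile at each of four fire points and sets the game state to NewEnumerator1.
; Separate left/right axis values feed only disconnected rotation logic.
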(event EventBeginPlay
  (Variables|Default|SetFire_Position (Utilities|Array|MakeArray (Variables|Default|GetFirePosition1) (Variables|Default|GetFirePosition2) (Variables|Default|GetFirePosition3) (Variables|Default|GetFirePosition0))))

(event Collision|EventActorBeginOverlap
  (params (OtherActor :type Actor%20Object%20Reference)))

(event EventTick
  (params (DeltaSeconds :type Float%20%28single-precision%29))
  (Transformation|AddLocalRotation (Variables|Default|GetMotiongun_Base) (Math|Rotator|MakeRotator 0.0 0.0 (* DeltaSeconds (Variables|Default|GetPlayer_Speed) (Input|AxisValues|GetPawn_Rotation))) false false)
  (Transformation|SetWorldRotation (Variables|Default|GetMotiongun_Base) (Utilities|MacroClampRotationBlock) false false))

(event Input|ActionEvents|InputActionPawn_Fire
  (params (Key :type Key%20Structure :default "None"))
  (:Pressed
    (Audio|Components|Audio|Play (Variables|Default|GetAudio) 0.0)
    (for _array_element (Variables|Default|GetFire_Position)
      (Game|SpawnActorfromClass "/Game/Blueprints/BP_Missile.BP_Missile_C" (Transformation|GetWorldTransform _array_element) "Undefined" 0 0)
      (bind _asmy_game_state_base_1 (Utilities|Casting|CastToMyGameStateBase1 (Game|GetGameState)))
      (Variables|/Game/Blueprints/WorldSettings/MyGameStateBase1.MyGameStateBase1_C|Set현재게임상태 _asmy_game_state_base_1 "NewEnumerator1"))))

(event Input|AxisEvents|InputAxisPawn_Rotation
  (params (AxisValue :type Float%20%28single-precision%29))
  ;[0.1763 1 0.2049] 입력축 회전
)

(event Input|AxisEvents|InputAxisPawn_Rotation_R
  (params (AxisValue :type Float%20%28single-precision%29))
  ;[1 0.01458 0] 오른쪽 30도 만큼만 회전
  (Variables|Default|SetAxis%20Value_RR AxisValue))

(event Input|AxisEvents|InputAxisPawn_Rotation_L
  (params (AxisValue :type Float%20%28single-precision%29))
  ;[0.08993 0.1404 1] 왼쪽 30도 만큼만 회전
  (Variables|Default|SetAxis%20Value_RL AxisValue))

(fn ConstructionScript)