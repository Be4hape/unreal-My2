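; BP_Target is a target actor that reports the elemental damage it takes.
; On AnyDamage it casts the damage type to BP_DamageType, passes fixed fire and poison resistances to its 속성피해적용 (apply elemental damage) function, and prints the result as total missile damage.
; Game-state change, missile-tag check, debug print and HP-decrement-then-destroy logic remain as disconnected nodes, so damage never reduces HP or destroys the target here.
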(event EventBeginPlay)

(event Collision|EventActorBeginOverlap
  (params (OtherActor :type Actor%20Object%20Reference)))

(event EventTick
  (params (DeltaSeconds :type Float%20%28single-precision%29)))

(event Collision|EventActorEndOverlap
  (params (OtherActor :type Actor%20Object%20Reference)))

(event Game|Damage|EventAnyDamage
  (params (Damage :type Float%20%28single-precision%29) (DamageType :type Damage%20Type%20Object%20Reference) (InstigatedBy :type Controller%20Object%20Reference) (DamageCauser :type Actor%20Object%20Reference))
  (bind _asbp_damage_type (Utilities|Casting|CastToBP_DamageType DamageType))
  (bind _전체속성피해 (Default|속성피해적용 _asbp_damage_type 5.0 5.0))
  (Development|PrintText (Utilities|Text|FormatText "미사일 전체 속성피해 {d}" _전체속성피해)))

(fn ConstructionScript)